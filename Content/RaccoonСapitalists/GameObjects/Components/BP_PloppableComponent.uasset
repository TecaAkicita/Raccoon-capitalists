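; BP_PloppableComponent is an actor component that validates where its owning placeable object sits and previews the result through materials.
; On BeginPlay and on the owner's overlap begin/end events, it asks BP_GridManager whether the closest grid cell is free.
; A cost check through GM_GameModeBase also invalidates unaffordable BP_BasePlaceableAsset owners.
; It then sets the first material slot of each static mesh to the valid or invalid ploppable material.
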(event Custom|OverlapStatusChanged
  (params (OverlappedActor :type Actor%20Object%20Reference) (OtherActor :type Actor%20Object%20Reference))
  (CallFunction|UpadateState))

(event EventBeginPlay
  (bind _returnvalue (Components|GetOwner))
  (Collision|BindEventtoOnActorBeginOverlap _returnvalue (delegate Custom|OverlapStatusChanged))
  (Collision|BindEventtoOnActorEndOverlap _returnvalue (delegate Custom|OverlapStatusChanged))
  (CallFunction|UpadateState))

(fn UpadateState
  (bind _returnvalue (Actor|GetActorOfClass "/Game/RaccoonСapitalists/GameObjects/Grid/BP_GridManager.BP_GridManager_C"))
  (bind _output (Default|GetClosesGridCell _returnvalue (Transformation|GetActorLocation (Components|GetOwner))))
  (bind _output_get (Variables|Default|SetIsPlacementValid (not (Variables|/Game/RaccoonСapitalists/GameObjects/Grid/BP_GridCell.BP_GridCell_C|GetIsOccupied _output))))
  (CallFunction|CostCheck)
  (for _array_element (Actor|GetComponentsByClass (Components|GetOwner) "/Script/Engine.StaticMeshComponent")
    (if _output_get
      (Rendering|Material|SetMaterial _array_element 0 (Variables|Default|GetPloppableMaterial))
      (else
        (Rendering|Material|SetMaterial _array_element 0 (Variables|Default|GetInvalidPloppableMaterial))))))

(fn CostCheck
  (bind _asbp_base_placeable_asset (Utilities|Casting|CastToBP_BasePlaceableAsset (Components|GetOwner)))
  (bind _asgm_game_mode_base (Utilities|Casting|CastToGM_GameModeBase (Game|GetGameMode)))
  (bind _canafford (Default|CanAffordObject _asgm_game_mode_base (Variables|/Game/RaccoonСapitalists/GameObjects/Objects/BP_BasePlaceableAsset.BP_BasePlaceableAsset_C|GetCostOfObjects _asbp_base_placeable_asset)))
  (if (not _canafford)
    (Variables|Default|SetIsPlacementValid false)))