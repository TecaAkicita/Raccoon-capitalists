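; BP_GridManager builds a square grid of BP_GridCell actors centred on the world origin and answers nearest-cell queries.
; On BeginPlay it spawns GridSize squared cells spaced by WorldGridSize into a flat, row-by-row GridArray.
; It then links each cell's four compass neighbours through index arithmetic, with North/South along X and East/West along Y.
; Lookup functions linearly scan the array by distance for the closest cell or its position.
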(event EventBeginPlay
  (CallFunction|PopulateGrid)
  (CallFunction|PopulteGridCellNeighbours))

(fn ConstructionScript)

(fn PopulateGrid
  (bind _worldgridsize (Variables|Default|GetWorldGridSize))
  (bind _worldgridsize_2 (Variables|Default|GetWorldGridSize))
  (Utilities|Array|Clear (Variables|Default|GetGridArray))
  (LocalVariables|SetWorldOffset (- (* (* (Variables|Default|GetGridSize) _worldgridsize) 0.5) (* _worldgridsize 0.5)))
  ;[0.15 0.15 0.15 0.5] Y
  (for _index (range 0 (- (Variables|Default|GetGridSize) 1))
    ;[0.15 0.15 0.15 0.5] X
    (for _index_2 (range 0 (- (Variables|Default|GetGridSize) 1))
      (bind _returnvalue (Game|SpawnActorfromClass "/Game/RaccoonСapitalists/GameObjects/Grid/BP_GridCell.BP_GridCell_C" (Math|Transform|MakeTransform (Math|Vector|MakeVector (- (* _index_2 _worldgridsize_2) (LocalVariables|GetWorldOffset)) (- (* _worldgridsize_2 _index) (LocalVariables|GetWorldOffset)) 0.0)) "AlwaysSpawn" "MultiplyWithRoot" 0 0))
      (Utilities|Array|Add (Variables|Default|GetGridArray) _returnvalue))))

(fn GetClosesGridPosition
  (params (InPosition :type Vector))
  (bind _gridarray (Variables|Default|GetGridArray))
  (bind _output (Utilities|Array|Get(acopy) _gridarray))
  (bind _returnvalue (Transformation|GetActorLocation _output))
  (LocalVariables|SetClosesPosition _returnvalue)
  (LocalVariables|SetClosesDistance (Math|Vector|Distance(Vector) InPosition _returnvalue))
  (for _array_element (Variables|Default|GetGridArray)
    (if (< (Math|Vector|Distance(Vector) (Transformation|GetActorLocation _array_element) InPosition) (LocalVariables|GetClosesDistance))
      (LocalVariables|SetClosesPosition (Transformation|GetActorLocation _array_element))
      (LocalVariables|SetClosesDistance (Math|Vector|Distance(Vector) (Transformation|GetActorLocation _array_element) InPosition))))
  (return (LocalVariables|GetClosesPosition)))

(fn PopulteGridCellNeighbours
  (bind _gridarray (Variables|Default|GetGridArray))
  (for (_array_element _array_index) (Variables|Default|GetGridArray)
    ;[0.15 0.15 0.15 0.5] западный сосед
    (if (>= (- _array_index (Variables|Default|GetGridSize)) 0)
      (Variables|/Game/RaccoonСapitalists/GameObjects/Grid/BP_GridCell.BP_GridCell_C|SetNeighbourWest _array_element (Utilities|Array|Get(acopy) (Variables|Default|GetGridArray) (- _array_index (Variables|Default|GetGridSize)))))
    ;[0.15 0.15 0.15 0.5] восточный сосед
    (if (< (+ _array_index (Variables|Default|GetGridSize)) (Utilities|Array|Length _gridarray))
      (Variables|/Game/RaccoonСapitalists/GameObjects/Grid/BP_GridCell.BP_GridCell_C|SetNeighbourEast _array_element (Utilities|Array|Get(acopy) _gridarray (+ _array_index (Variables|Default|GetGridSize)))))
    ;[0.15 0.15 0.15 0.5] южный сосед
    (if (or (== _array_index 0) (== (Math|Integer|%(Integer) _array_index (Variables|Default|GetGridSize)) 0))
      _
      (else
        (Variables|/Game/RaccoonСapitalists/GameObjects/Grid/BP_GridCell.BP_GridCell_C|SetNeighbourSouth _array_element (Utilities|Array|Get(acopy) (Variables|Default|GetGridArray) (- _array_index 1)))))
    ;[0.15 0.15 0.15 0.5] северный сосед
    (if (not (== (Math|Integer|%(Integer) (+ _array_index 1) (Variables|Default|GetGridSize)) 0))
      (Variables|/Game/RaccoonСapitalists/GameObjects/Grid/BP_GridCell.BP_GridCell_C|SetNeighbourNorth _array_element (Utilities|Array|Get(acopy) (Variables|Default|GetGridArray) (+ _array_index 1))))))

(fn GetClosesGridCell
  (params (InPosition :type Vector))
  (LocalVariables|SetClosesDistance (Math|Vector|Distance(Vector) InPosition (Transformation|GetActorLocation (Utilities|Array|Get(acopy) (Variables|Default|GetGridArray)))))
  (for (_array_element _array_index) (Variables|Default|GetGridArray)
    (if (< (Math|Vector|Distance(Vector) (Transformation|GetActorLocation _array_element) InPosition) (LocalVariables|GetClosesDistance))
      (LocalVariables|SetClosesDistance (Math|Vector|Distance(Vector) (Transformation|GetActorLocation _array_element) InPosition))
      (LocalVariables|SetArrayIndex _array_index)))
  (return (Utilities|Array|Get(acopy) (Variables|Default|GetGridArray) (LocalVariables|GetArrayIndex))))