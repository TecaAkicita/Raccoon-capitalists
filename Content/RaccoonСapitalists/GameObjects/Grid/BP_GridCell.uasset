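; BP_GridCell is a grid cell actor that tracks whether it is occupied by a building.
; SetOccupied flags the cell as occupied and stores the building type and occupying actor.
; The cell references its north, east, west and south neighbours, and a debug event paints its cube red.
; The calls that would trigger that highlight on the neighbours are disconnected and never run.
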(event Custom|SetOccupied
  (params (New%20Building%20Type :type E_BuildingType%20Enum :default "NewEnumerator2") (Occupying%20Actor%20Ref :type Actor%20Object%20Reference))
  (Variables|Default|SetIsOccupied true)
  (Variables|Default|SetOccupyingType New%20Building%20Type)
  (Variables|Default|SetOccupingActor Occupying%20Actor%20Ref))

(event Custom|DebugShowNeighbourOccupied
  ;[0.15 0.15 0.15 0.5] Debug
  (Rendering|Material|SetMaterial (Variables|Default|GetCube) 0 "/Game/RaccoonСapitalists/MaterialLibrary/Debug/M_Red_DEBUG.M_Red_DEBUG"))

(event EventBeginPlay)

(event Collision|EventActorBeginOverlap
  (params (OtherActor :type Actor%20Object%20Reference)))

(event EventTick
  (params (DeltaSeconds :type Float%20%28single-precision%29)))

(fn ConstructionScript)