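; Player controller for grid-based building placement that also forwards camera orbit, movement and zoom input to the CB_CameraController pawn.
; In placement mode, it spawns a preview actor and each tick snaps it to BP_GridManager's closest position under a mouse trace.
; Left click spawns the building if BP_PloppableComponent validates it, occupies the cell and reports its cost to GM_GameModeBase.
; OnPlacementInfoUpdated swaps the preview type or exits placement mode.
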(event Custom|OnPlacementInfoUpdated
  (params (InPlacebleActorType :type BP%20Base%20Placeable%20Asset%20Class%20Reference) (InPlacebleMode :type E_BuildingType%20Enum :default "NewEnumerator2"))
  (bind _placebleactor (Variables|Default|GetPlacebleActor))
  (Variables|Default|SetPlacebleActorType InPlacebleActorType)
  (bind _output_get (Variables|Default|SetPlaceableBuildingType InPlacebleMode))
  (if (Utilities|Enum|Equal(Enum) _output_get "NewEnumerator2")
    (CallFunction|SetPlacebleModeEnabled false)
    (else
      (Utilities|IsValid _placebleactor
        (:Is%20Valid
          (Actor|DestroyActor _placebleactor))
        (:Is%20Not%20Valid
          _))
      (CallFunction|RefreshPlacebleBuilding)
      (CallFunction|SetPlacebleModeEnabled true))))

(event EventBeginPlay
  (CallFunction|SetPlacebleModeEnabled true))

(event EventTick
  (params (DeltaSeconds :type Float%20%28single-precision%29))
  (if (Variables|Default|GetPlacementModeEnabled)
    (CallFunction|UpdatePlacement)))

(event Input|ActionEvents|InputActionCameraZoomIn
  (params (Key :type Key%20Structure :default "None"))
  ;[0.15 0.15 0.15 0.5] Приблежение/отдаление камеры
  (:Pressed
    (bind _ascb_camera_controller (Utilities|Casting|CastToCB_CameraController (Pawn|GetControlledPawn)))
    (Default|CameraZoom _ascb_camera_controller -1.0)))

(event Input|ActionEvents|InputActionCameraZoomOut
  (params (Key :type Key%20Structure :default "None"))
  ;[0.15 0.15 0.15 0.5] Приблежение/отдаление камеры
  (:Pressed
    (bind _ascb_camera_controller (Utilities|Casting|CastToCB_CameraController (Pawn|GetControlledPawn)))
    (Default|CameraZoom _ascb_camera_controller 1.0)))

(event Input|ActionEvents|InputActionMouseLeftClick
  (params (Key :type Key%20Structure :default "None"))
  (:Pressed
    (if (Variables|Default|GetPlacementModeEnabled)
      (CallFunction|SpawnBuilding))))

(event Input|AxisEvents|InputAxisCameraOrbit
  (params (AxisValue :type Float%20%28single-precision%29))
  ;[0.15 0.15 0.15 0.5] Вращение камеры
  (bind _ascb_camera_controller (Utilities|Casting|CastToCB_CameraController (Pawn|GetControlledPawn)))
  (Default|CameraOrbit _ascb_camera_controller AxisValue))

(event Input|AxisEvents|InputAxisMoveForward/Backward
  (params (AxisValue :type Float%20%28single-precision%29))
  ;[0.15 0.15 0.15 0.5] Движение
  (bind _ascb_camera_controller (Utilities|Casting|CastToCB_CameraController (Pawn|GetControlledPawn)))
  (Default|MoveForward _ascb_camera_controller AxisValue))

(event Input|AxisEvents|InputAxisStrafeLeft/Right
  (params (AxisValue :type Float%20%28single-precision%29))
  ;[0.15 0.15 0.15 0.5] Движение
  (bind _ascb_camera_controller (Utilities|Casting|CastToCB_CameraController (Pawn|GetControlledPawn)))
  (Default|LeftRightStrafe _ascb_camera_controller AxisValue))

(fn ConstructionScript)

(fn SetPlacebleModeEnabled
  (params (IsEnable :type Boolean))
  (bind _placebleactor (Variables|Default|GetPlacebleActor))
  (if (== IsEnable (Variables|Default|GetPlacementModeEnabled))
    (return)
    (else
      (bind _output_get (Variables|Default|SetPlacementModeEnabled IsEnable))
      (if _output_get
        (CallFunction|RefreshPlacebleBuilding)
        (else
          (Utilities|IsValid _placebleactor
            (:Is%20Valid
              (Actor|DestroyActor _placebleactor))))))))

(fn UpdatePlacement
  (bind (_worldlocation _worlddirection) (Game|Player|ConvertMouseLocationToWorldSpace))
  (bind _outhit (Collision|LineTraceByChannel _worldlocation (+ _worldlocation (* _worlddirection 1e+04)) "TraceTypeQuery3" false 0 "None"))
  (if (.bBlockingHit (Collision|BreakHitResult _outhit))
    (bind _returnvalue (Actor|GetActorOfClass "/Game/RaccoonСapitalists/GameObjects/Grid/BP_GridManager.BP_GridManager_C"))
    (bind _outputvector (Default|GetClosesGridPosition _returnvalue (.Location (Collision|BreakHitResult _outhit))))
    (Transformation|SetActorLocation (Variables|Default|GetPlacebleActor) _outputvector false false)))

(fn SpawnBuilding
  (bind _placebleactor (Variables|Default|GetPlacebleActor))
  (bind _placebleactor_2 (Variables|Default|GetPlacebleActor))
  (bind _returnvalue (Actor|GetComponentbyClass _placebleactor "/Game/RaccoonСapitalists/GameObjects/Components/BP_PloppableComponent.BP_PloppableComponent_C"))
  (Utilities|IsValid _returnvalue
    (:Is%20Valid
      (if (Variables|/Game/RaccoonСapitalists/GameObjects/Components/BP_PloppableComponent.BP_PloppableComponent_C|GetIsPlacementValid _returnvalue)
        (bind _returnvalue_2 (Game|SpawnActorfromClass (Variables|Default|GetPlacebleActorType) (Transformation|GetActorTransform _placebleactor_2) "AlwaysSpawn" "MultiplyWithRoot" 0 0))
        (bind _returnvalue_3 (Actor|GetActorOfClass "/Game/RaccoonСapitalists/GameObjects/Grid/BP_GridManager.BP_GridManager_C"))
        (bind _output (Default|GetClosesGridCell _returnvalue_3 (Transformation|GetActorLocation _placebleactor_2)))
        (bind _asbp_base_placeable_asset (Utilities|Casting|CastToBP_BasePlaceableAsset _returnvalue_2))
        (Variables|/Game/RaccoonСapitalists/GameObjects/Objects/BP_BasePlaceableAsset.BP_BasePlaceableAsset_C|SetGridCellRef _asbp_base_placeable_asset _output)
        (Default|SetOccupied _output (Variables|/Game/RaccoonСapitalists/GameObjects/Objects/BP_BasePlaceableAsset.BP_BasePlaceableAsset_C|GetBuildingType _asbp_base_placeable_asset) _returnvalue_2)
        ;[0.15 0.15 0.15 0.5] Buy objects
        (bind _asgm_game_mode_base (Utilities|Casting|CastToGM_GameModeBase (Game|GetGameMode)))
        (Default|ObjectBought _asgm_game_mode_base (Variables|/Game/RaccoonСapitalists/GameObjects/Objects/BP_BasePlaceableAsset.BP_BasePlaceableAsset_C|GetCostOfObjects _asbp_base_placeable_asset))))))

(fn RefreshPlacebleBuilding
  (bind _returnvalue (Game|SpawnActorfromClass (Variables|Default|GetPlacebleActorType) (Math|Transform|MakeTransform "0.000000,0.000000,-100000.000000") "AlwaysSpawn" "MultiplyWithRoot" 0 0))
  (bind _asbp_base_placeable_asset (Utilities|Casting|CastToBP_BasePlaceableAsset _returnvalue)
    (:then
      (bind _output_get (Variables|Default|SetPlacebleActor _asbp_base_placeable_asset))
      (Utilities|IsValid (Actor|GetComponentbyClass _output_get "/Game/RaccoonСapitalists/GameObjects/Components/BP_ClickableComponent.BP_ClickableComponent_C")
        (:Is%20Valid
          (Default|InPlacebleMode (Actor|GetComponentbyClass _output_get "/Game/RaccoonСapitalists/GameObjects/Components/BP_ClickableComponent.BP_ClickableComponent_C")))
        (:Is%20Not%20Valid
          _))
      (AddComponent|AddBPPloppableComponent _output_get))
    (:CastFailed
      (Class|AutomationBlueprintFunctionLibrary|AddExpectedLogError "Actor of non-placeable building type detected in SetPlacebleModeEnabled"))))