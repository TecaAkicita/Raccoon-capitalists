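; Main player controller that routes keyboard and mouse input into the game's building placement system.
; On BeginPlay it adds the Enhanced Input mapping context and, behind the same subsystem validity check, spawns and stores a building manager actor.
; Hardcoded key events, rather than input actions, tell the manager to spawn square buildings of different sizes, rotate, delete or handle mouse clicks, each printing a debug string.
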(event EventBeginPlay
  (bind _returnvalue (PlayerController|LocalPlayerSubsystems|GetEnhancedInputLocalPlayerSubsystem))
  (Utilities|IsValid _returnvalue
    (:Is%20Valid
      (Input|AddMappingContext _returnvalue "/Game/RaccoonСapitalists/Input/InputMappingContext.InputMappingContext" 0 "(bIgnoreAllPressedKeysUntilRelease=True,bForceImmediately=False,bNotifyUserSettings=False)")
      (bind _returnvalue_2 (Game|SpawnActorfromClass "/Game/RaccoonСapitalists/Blueprints/BuildingSystem/Bp_BuildingManager.Bp_BuildingManager_C" (Math|Transform|MakeTransform "0, 0, 0" "0, 0, 0" "1.000000,1.000000,1.000000") "Undefined" "MultiplyWithRoot" 0 0))
      (Variables|Default|SetBuildManager _returnvalue_2))))

(event EventTick
  (params (DeltaSeconds :type Float%20%28single-precision%29)))

(event Input|KeyboardEvents|1
  (params (Key :type Key%20Structure :default "None"))
  (:Pressed
    (Default|SpawnandAttachBuilding (Variables|Default|GetBuildManager) "/Game/RaccoonСapitalists/Blueprints/BuildingSystem/Buildings/BP_Building_Square1x1.BP_Building_Square1x1_C" "NewEnumerator0")
    (Development|PrintString "key 1")))

(event Input|KeyboardEvents|2
  (params (Key :type Key%20Structure :default "None"))
  (:Pressed
    (Default|SpawnandAttachBuilding (Variables|Default|GetBuildManager) "/Game/RaccoonСapitalists/Blueprints/BuildingSystem/Buildings/BP_Building_Square2x2.BP_Building_Square2x2_C" "NewEnumerator1")
    (Development|PrintString "key 2")))

(event Input|KeyboardEvents|R
  (params (Key :type Key%20Structure :default "None"))
  (:Pressed
    (Default|HandleRotateKey (Variables|Default|GetBuildManager))
    (Development|PrintString "key R")))

(event Input|MouseEvents|LeftMouseButton
  (params (Key :type Key%20Structure :default "None"))
  (:Pressed
    (Default|HandleLeftClick (Variables|Default|GetBuildManager))
    (Development|PrintString "key Left")))

(event Input|MouseEvents|RightMouseButton
  (params (Key :type Key%20Structure :default "None"))
  (:Pressed
    (Default|HandleRightClick (Variables|Default|GetBuildManager))
    (Development|PrintString "key Right")))

(event Input|KeyboardEvents|3
  (params (Key :type Key%20Structure :default "None"))
  (:Pressed
    (Default|SpawnandAttachBuilding (Variables|Default|GetBuildManager) "/Game/RaccoonСapitalists/Blueprints/BuildingSystem/Buildings/BP_Building_Square3x3.BP_Building_Square3x3_C" "NewEnumerator2")
    (Development|PrintString "key 3")))

(event Input|KeyboardEvents|5
  (params (Key :type Key%20Structure :default "None"))
  (:Pressed
    (Default|SpawnandAttachBuilding (Variables|Default|GetBuildManager) "/Game/RaccoonСapitalists/Blueprints/BuildingSystem/Buildings/BP_Building_Square5x5.BP_Building_Square5x5_C" "NewEnumerator3")
    (Development|PrintString "key 5")))

(event Input|KeyboardEvents|F
  (params (Key :type Key%20Structure :default "None"))
  (:Pressed
    (Default|HandleDelete (Variables|Default|GetBuildManager))
    (Development|PrintString "key D")))

(fn ConstructionScript)