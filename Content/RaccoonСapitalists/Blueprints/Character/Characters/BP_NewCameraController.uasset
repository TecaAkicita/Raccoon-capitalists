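; Camera controller built on character movement, providing planar movement, yaw orbit and spring-arm zoom.
; Forward and strafe inputs move along the control rotation's yaw only, while orbit input adds controller yaw scaled by orbital speed.
; Zoom changes the spring arm length within set limits, then rescales walk speed by arm length over minimum zoom, so movement is faster when zoomed out.
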(event Custom|CameraOrbit
  (params (Magnitude :type Float%20%28double-precision%29))
  ;[0.15 0.15 0.15 0.5] Вращение камеры
  (Pawn|Input|AddControllerYawInput (* Magnitude (Variables|Default|GetOrbitalSpeed))))

(event Custom|MoveForward
  (params (Magnitude :type Float%20%28double-precision%29))
  ;[0.15 0.15 0.15 0.5] Движение
  (Pawn|Input|AddMovementInput (Math|Vector|GetForwardVector (Math|Rotator|MakeRotator 0.0 0.0 (.Yaw (Math|Rotator|BreakRotator (Pawn|GetControlRotation :!class /Script/Engine.Pawn))))) Magnitude false))

(event Custom|LeftRightStrafe
  (params (Magnitude :type Float%20%28double-precision%29))
  ;[0.15 0.15 0.15 0.5] Движение
  (Pawn|Input|AddMovementInput (Math|Vector|GetRightVector (Math|Rotator|MakeRotator 0.0 0.0 (.Yaw (Math|Rotator|BreakRotator (Pawn|GetControlRotation :!class /Script/Engine.Pawn))))) Magnitude false))

(event Custom|CameraZoom
  (params (Magnitude :type Float%20%28double-precision%29))
  (bind _springarm (Variables|Default|GetSpringArm))
  ;[0.15 0.15 0.15 0.5] Приблежение/отдаление камеры
  (Variables|/Script/Engine.SpringArmComponent|SetTargetArmLength _springarm (Math|Float|Clamp(Float) (+ (* Magnitude (Variables|Default|GetZoomSpeed)) (Variables|/Script/Engine.SpringArmComponent|GetTargetArmLength _springarm)) (Variables|Default|GetMinZoom) (Variables|Default|GetMaxZoom)))
  (CallFunction|UpdateMovementSpeed))

(event EventBeginPlay
  (Variables|Default|SetInitialMovemetSpeed (Variables|/Script/Engine.CharacterMovementComponent|GetMaxWalkSpeed (Variables|Character|GetCharacterMovement)))
  (CallFunction|UpdateMovementSpeed))

(fn ConstructionScript)

(fn UpdateMovementSpeed
  (Variables|/Script/Engine.CharacterMovementComponent|SetMaxWalkSpeed (Variables|Character|GetCharacterMovement) (* (Variables|Default|GetInitialMovemetSpeed) (/ (Variables|/Script/Engine.SpringArmComponent|GetTargetArmLength (Variables|Default|GetSpringArm)) (Variables|Default|GetMinZoom)))))