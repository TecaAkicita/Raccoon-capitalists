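; Player controller that handles camera control and building placement input.
; Orbit, movement, strafe and zoom inputs are forwarded to the possessed BP_CameraController pawn.
; On BeginPlay it spawns a Bp_BuildingManager, which receives hardcoded key and mouse events for spawning two building types, rotating, deleting and handling left and right clicks.
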(event EventBeginPlay
  (bind _returnvalue (Game|SpawnActorfromClass "/Game/RaccoonСapitalists/Blueprints/BuildingSystem/Bp_BuildingManager.Bp_BuildingManager_C" (Math|Transform|MakeTransform "0, 0, 0" "0, 0, 0" "1.000000,1.000000,1.000000") "Undefined" "MultiplyWithRoot" 0 0))
  (Variables|Default|SetBuildManager _returnvalue))

(event EventTick
  (params (DeltaSeconds :type Float%20%28single-precision%29)))

(event Input|ActionEvents|InputActionCameraZoomIn
  (params (Key :type Key%20Structure :default "None"))
  ;[0.15 0.15 0.15 0.5] Приблежение/отдаление камеры
  (:Pressed
    (bind _asbp_camera_controller (Utilities|Casting|CastToBP_CameraController (Pawn|GetControlledPawn)))
    (Default|CameraZoom _asbp_camera_controller -1.0)))

(event Input|ActionEvents|InputActionCameraZoomOut
  (params (Key :type Key%20Structure :default "None"))
  ;[0.15 0.15 0.15 0.5] Приблежение/отдаление камеры
  (:Pressed
    (bind _asbp_camera_controller (Utilities|Casting|CastToBP_CameraController (Pawn|GetControlledPawn)))
    (Default|CameraZoom _asbp_camera_controller 1.0)))

(event Input|AxisEvents|InputAxisCameraOrbit
  (params (AxisValue :type Float%20%28single-precision%29))
  ;[0.15 0.15 0.15 0.5] Вращение камеры
  (bind _asbp_camera_controller (Utilities|Casting|CastToBP_CameraController (Pawn|GetControlledPawn)))
  (Default|CameraOrbit _asbp_camera_controller AxisValue))

(event Input|AxisEvents|InputAxisMoveForward/Backward
  (params (AxisValue :type Float%20%28single-precision%29))
  ;[0.15 0.15 0.15 0.5] Движение
  (bind _asbp_camera_controller (Utilities|Casting|CastToBP_CameraController (Pawn|GetControlledPawn)))
  (Default|MoveForward _asbp_camera_controller AxisValue))

(event Input|AxisEvents|InputAxisStrafeLeft/Right
  (params (AxisValue :type Float%20%28single-precision%29))
  ;[0.15 0.15 0.15 0.5] Движение
  (bind _asbp_camera_controller (Utilities|Casting|CastToBP_CameraController (Pawn|GetControlledPawn)))
  (Default|LeftRightStrafe _asbp_camera_controller AxisValue))

(event Input|KeyboardEvents|1
  (params (Key :type Key%20Structure :default "None"))
  (:Released
    (Default|SpawnandAttachBuilding (Variables|Default|GetBuildManager) 0 "NewEnumerator0")))

(event Input|KeyboardEvents|2
  (params (Key :type Key%20Structure :default "None"))
  (:Released
    (Default|SpawnandAttachBuilding (Variables|Default|GetBuildManager) 0 "NewEnumerator1")))

(event Input|KeyboardEvents|R
  (params (Key :type Key%20Structure :default "None"))
  (:Released
    (Default|HandleRotateKey (Variables|Default|GetBuildManager))))

(event Input|MouseEvents|LeftMouseButton
  (params (Key :type Key%20Structure :default "None"))
  (:Pressed
    (Default|HandleLeftClick (Variables|Default|GetBuildManager))))

(event Input|KeyboardEvents|D
  (params (Key :type Key%20Structure :default "None"))
  (:Released
    (Default|HandleDelete (Variables|Default|GetBuildManager))))

(event Input|MouseEvents|RightMouseButton
  (params (Key :type Key%20Structure :default "None"))
  (:Pressed
    (Default|HandleRightClick (Variables|Default|GetBuildManager))))

(fn ConstructionScript)