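; Test player controller that drives building placement through a spawned Bp_BuildingManager.
; On BeginPlay it spawns the manager and keeps a reference to it.
; Number keys spawn and attach a basic pipe or a 2x2 square building, while R, mouse clicks and D forward rotate, click and delete actions to the manager.
; Each input also prints a debug string.
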(event EventBeginPlay
  (bind _returnvalue (Game|SpawnActorfromClass "/Game/RaccoonСapitalists/Blueprints/BuildingSystem/Bp_BuildingManager.Bp_BuildingManager_C" (Math|Transform|MakeTransform "0, 0, 0" "0, 0, 0" "1.000000,1.000000,1.000000") "Undefined" "MultiplyWithRoot" 0 0))
  (Variables|Default|SetBuildManager _returnvalue))

(event EventTick
  (params (DeltaSeconds :type Float%20%28single-precision%29)))

(event Input|KeyboardEvents|1
  (params (Key :type Key%20Structure))
  (:Pressed
    (Default|SpawnandAttachBuilding (Variables|Default|GetBuildManager) "/Game/RaccoonСapitalists/Blueprints/BuildingSystem/Buildings/BP_Building_BasicPipe.BP_Building_BasicPipe_C" "NewEnumerator0")
    (Development|PrintString "key 1")))

(event Input|KeyboardEvents|2
  (params (Key :type Key%20Structure))
  (:Pressed
    (Default|SpawnandAttachBuilding (Variables|Default|GetBuildManager) "/Game/RaccoonСapitalists/Blueprints/BuildingSystem/Buildings/BP_Building_Square2x2.BP_Building_Square2x2_C" "NewEnumerator1")
    (Development|PrintString "key 2")))

(event Input|KeyboardEvents|D
  (params (Key :type Key%20Structure))
  (:Pressed
    (Default|HandleDelete (Variables|Default|GetBuildManager))
    (Development|PrintString "key D")))

(event Input|KeyboardEvents|R
  (params (Key :type Key%20Structure))
  (:Pressed
    (Default|HandleRotateKey (Variables|Default|GetBuildManager))
    (Development|PrintString "key R")))

(event Input|MouseEvents|LeftMouseButton
  (params (Key :type Key%20Structure))
  (:Pressed
    (Default|HandleLeftClick (Variables|Default|GetBuildManager))
    (Development|PrintString "key Left")))

(event Input|MouseEvents|RightMouseButton
  (params (Key :type Key%20Structure))
  (:Pressed
    (Default|HandleRightClick (Variables|Default|GetBuildManager))
    (Development|PrintString "key Right")))

(fn ConstructionScript)