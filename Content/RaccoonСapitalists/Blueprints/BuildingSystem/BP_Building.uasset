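; BP_Building is a building actor that supplies its grid footprint and shows its state through materials.
; It creates a BP_ShapeHelper on BeginPlay and starts with a ghost material.
; GetFootPrint takes the base square shape for its BuildingType from the helper and repeatedly rotates it according to CurrentRotation in 90-degree steps.
; Separate functions switch the mesh to a solid material or toggle between selected and solid.
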(event EventBeginPlay
  (bind _returnvalue (Game|ConstructObjectfromClass "/Game/RaccoonСapitalists/Blueprints/BuildingSystem/BP_ShapeHelper.BP_ShapeHelper_C"))
  (Variables|Default|SetShapeHelper _returnvalue)
  (Rendering|Material|SetMaterial (Variables|Default|GetStaticMesh) 0 "/Game/RaccoonСapitalists/Assets/Materials/BuildingSystem/M_BuildingGhost.M_BuildingGhost"))

(event Collision|EventActorBeginOverlap
  (params (OtherActor :type Actor%20Object%20Reference)))

(event EventTick
  (params (DeltaSeconds :type Float%20%28single-precision%29)))

(fn ConstructionScript)

(fn SetSelected
  (params (Condition :type Boolean))
  (if Condition
    (Rendering|Material|SetMaterial (Variables|Default|GetStaticMesh) 0 "/Game/RaccoonСapitalists/Assets/Materials/BuildingSystem/M_BuildingSelect.M_BuildingSelect")
    (else
      (Rendering|Material|SetMaterial (Variables|Default|GetStaticMesh) 0 "/Game/RaccoonСapitalists/Assets/Materials/BuildingSystem/M_BuildingSolid.M_BuildingSolid"))))

(fn GetFootPrint
  (switch Utilities|FlowControl|Switch|SwitchonE_BuildingType (Variables|Default|GetBuildingType)
    (:NewEnumerator0
      (LocalVariables|SetBaseFootPrint (Default|GetSquare1x1 (Variables|Default|GetShapeHelper))))
    (:NewEnumerator1
      (LocalVariables|SetBaseFootPrint (Default|GetSquare2x2 (Variables|Default|GetShapeHelper)))))
  (LocalVariables|SetRotateFootPrint (LocalVariables|GetBaseFootPrint))
  (for _index (range 0 (/ (Variables|Default|GetCurrentRotation) 90))
    (LocalVariables|SetRotateFootPrint (Default|GetRotate (Variables|Default|GetShapeHelper) (LocalVariables|GetRotateFootPrint))))
  (return (LocalVariables|GetRotateFootPrint)))

(fn SetSolidBuildingMaterial
  (Rendering|Material|SetMaterial (Variables|Default|GetStaticMesh) 0 "/Game/RaccoonСapitalists/Assets/Materials/BuildingSystem/M_BuildingSolid.M_BuildingSolid"))