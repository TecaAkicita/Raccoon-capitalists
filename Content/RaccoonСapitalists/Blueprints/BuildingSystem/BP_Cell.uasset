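; BP_Cell is a single cell in the building system, showing placement feedback through the color of its static mesh.
; SetCellState stores the current state and swaps the material: white for Idle, green for Can Place, red for both Cannot Place and Selected.
; SetOccupided only stores an occupancy flag; the cell has no active event logic, so both functions rely on external callers.
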(event EventBeginPlay)

(event Collision|EventActorBeginOverlap
  (params (OtherActor :type Actor%20Object%20Reference)))

(event EventTick
  (params (DeltaSeconds :type Float%20%28single-precision%29)))

(fn ConstructionScript)

(fn SetCellState
  (params (CurrentState :type E_CellState%20Enum :default "NewEnumerator0"))
  (bind _output_get (Variables|Default|SetCurrentState CurrentState))
  (switch Utilities|FlowControl|Switch|SwitchonE_CellState _output_get
    (:NewEnumerator0
      (Rendering|Material|SetMaterial (Variables|Default|GetStaticMesh) 0 "/Game/RaccoonСapitalists/Assets/Materials/BuildingSystem/M_CellWhite.M_CellWhite"))
    (:NewEnumerator1
      (Rendering|Material|SetMaterial (Variables|Default|GetStaticMesh) 0 "/Game/RaccoonСapitalists/Assets/Materials/BuildingSystem/M_CellGreen.M_CellGreen"))
    (:NewEnumerator2
      (Rendering|Material|SetMaterial (Variables|Default|GetStaticMesh) 0 "/Game/RaccoonСapitalists/Assets/Materials/BuildingSystem/M_CellRed.M_CellRed"))
    (:NewEnumerator3
      (Rendering|Material|SetMaterial (Variables|Default|GetStaticMesh) 0 "/Game/RaccoonСapitalists/Assets/Materials/BuildingSystem/M_CellRed.M_CellRed"))))

(fn SetOccupided
  (params (isOccupided :type Boolean))
  (Variables|Default|SetisOccupided isOccupided))