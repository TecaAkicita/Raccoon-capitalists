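; BP_ShapeHelper is a building-system helper that supplies grid footprints as arrays of integer cell offsets.
; GetShapeFootPrint maps a shape selection to one of four hardcoded square footprints, from 1x1 to 5x5, each anchored at a corner on (0,0).
; GetRotate turns any point array 90 degrees around that origin by mapping (X, Y) to (-Y, X), without shifting negative results back.
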(fn GetSquare1x1
  (return (Utilities|Array|MakeArray (Utilities|Struct|MakeIntPoint 0 0))))

(fn GetSquare2x2
  (return (Utilities|Array|MakeArray (Utilities|Struct|MakeIntPoint 0 0) (Utilities|Struct|MakeIntPoint 1 0) (Utilities|Struct|MakeIntPoint 0 1) (Utilities|Struct|MakeIntPoint 1 1))))

(fn GetSquare3x3
  (return (Utilities|Array|MakeArray (Utilities|Struct|MakeIntPoint 0 0) (Utilities|Struct|MakeIntPoint 1 0) (Utilities|Struct|MakeIntPoint 2 0) (Utilities|Struct|MakeIntPoint 0 1) (Utilities|Struct|MakeIntPoint 1 1) (Utilities|Struct|MakeIntPoint 2 1) (Utilities|Struct|MakeIntPoint 0 2) (Utilities|Struct|MakeIntPoint 1 2) (Utilities|Struct|MakeIntPoint 2 2))))

(fn GetSquare5x5
  (return (Utilities|Array|MakeArray (Utilities|Struct|MakeIntPoint 0 0) (Utilities|Struct|MakeIntPoint 1 0) (Utilities|Struct|MakeIntPoint 2 0) (Utilities|Struct|MakeIntPoint 3 0) (Utilities|Struct|MakeIntPoint 4 0) (Utilities|Struct|MakeIntPoint 0 1) (Utilities|Struct|MakeIntPoint 1 1) (Utilities|Struct|MakeIntPoint 2 1) (Utilities|Struct|MakeIntPoint 3 1) (Utilities|Struct|MakeIntPoint 4 1) (Utilities|Struct|MakeIntPoint 0 2) (Utilities|Struct|MakeIntPoint 1 2) (Utilities|Struct|MakeIntPoint 2 2) (Utilities|Struct|MakeIntPoint 3 2) (Utilities|Struct|MakeIntPoint 4 2) (Utilities|Struct|MakeIntPoint 0 3) (Utilities|Struct|MakeIntPoint 1 3) (Utilities|Struct|MakeIntPoint 2 3) (Utilities|Struct|MakeIntPoint 3 3) (Utilities|Struct|MakeIntPoint 4 3) (Utilities|Struct|MakeIntPoint 0 4) (Utilities|Struct|MakeIntPoint 1 4) (Utilities|Struct|MakeIntPoint 2 4) (Utilities|Struct|MakeIntPoint 3 4) (Utilities|Struct|MakeIntPoint 4 4))))

(fn GetRotate
  (params (NewParam :type Array%20of%20Int%20Point%20Structures))
  (for _array_element NewParam
    (Utilities|Array|Add (LocalVariables|GetOut) (Utilities|Struct|MakeIntPoint (* (.Y (Utilities|Struct|BreakIntPoint _array_element)) -1) (.X (Utilities|Struct|BreakIntPoint _array_element)))))
  (return (LocalVariables|GetOut)))

(fn GetShapeFootPrint
  (params (Selection :type E_BuildingType%20Enum :default "NewEnumerator0"))
  (switch Utilities|FlowControl|Switch|SwitchonE_BuildingType Selection
    (:NewEnumerator0
      (return (CallFunction|GetSquare1x1)))
    (:NewEnumerator1
      (return (CallFunction|GetSquare2x2)))
    (:NewEnumerator2
      (return (CallFunction|GetSquare3x3)))
    (:NewEnumerator3
      (return (CallFunction|GetSquare5x5)))))