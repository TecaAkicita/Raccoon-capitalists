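; BP_Building_BasicPipe is a pipe building in the building system that detects adjacent pipes and 3x3 buildings.
; Begin and end overlaps on its Box component set and clear the PipeConnected and BuildingConnected flags.
; An overlapping BP_Building_Square3x3 is stored as ConnectedBuilding and is not cleared on end overlap.
; An overlapping pipe is not stored; instead, that pipe's ConnectedPipe reference is set to None.
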(event OnComponentBeginOverlap(Box)
  (params (OverlappedComponent :type Primitive%20Component%20Object%20Reference) (OtherActor :type Actor%20Object%20Reference) (OtherComp :type Primitive%20Component%20Object%20Reference) (OtherBodyIndex :type Integer) (bFromSweep :type Boolean) (SweepResult :type Hit%20Result%20Structure%20%28by%20ref%29))
  (bind _asbp_building_basic_pipe (Utilities|Casting|CastToBP_Building_BasicPipe OtherActor)
    (:then
      (Variables|BP_Building_BasicPipe_C|SetConnectedPipe _asbp_building_basic_pipe 0)
      (Variables|Default|SetPipeConnected true))
    (:CastFailed
      (bind _asbp_building_square_3x_3 (Utilities|Casting|CastToBP_Building_Square3x3 OtherActor))
      (Variables|Default|SetConnectedBuilding _asbp_building_square_3x_3)
      (Variables|Default|SetBuildingConnected true))))

(event OnComponentEndOverlap(Box)
  (params (OverlappedComponent :type Primitive%20Component%20Object%20Reference) (OtherActor :type Actor%20Object%20Reference) (OtherComp :type Primitive%20Component%20Object%20Reference) (OtherBodyIndex :type Integer))
  (Utilities|Casting|CastToBP_Building_BasicPipe OtherActor
    (:then
      (Variables|Default|SetPipeConnected false))
    (:CastFailed
      (Utilities|Casting|CastToBP_Building_Square3x3 OtherActor)
      (Variables|Default|SetBuildingConnected false))))

(event EventBeginPlay
  (|CallParentFunction) ; This node is disabled and will not be called.\nDrag off pins to build functionality.
)

(event Collision|EventActorBeginOverlap
  (params (OtherActor :type Actor%20Object%20Reference))
  (|CallParentFunction OtherActor) ; This node is disabled and will not be called.\nDrag off pins to build functionality.
)

(event EventTick
  (params (DeltaSeconds :type Float%20%28single-precision%29))
  (|CallParentFunction DeltaSeconds) ; This node is disabled and will not be called.\nDrag off pins to build functionality.
)

(fn ConstructionScript
  (|CallParentFunction))