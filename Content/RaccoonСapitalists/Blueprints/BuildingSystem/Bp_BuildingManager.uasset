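; Grid-based building manager actor that handles placing, rotating, selecting and deleting buildings.
; On BeginPlay it spawns a centered grid of BP_Cell actors; while placing, Tick traces from the mouse and snaps the held building to cells.
; Footprint checks tint cells valid or invalid; committing marks them occupied and starts the building's resource generation.
; An Idle/Placing/Selecting state switch routes click, cancel, rotate and delete handlers.
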(event EventBeginPlay
  (CallFunction|InitalizeGrid))

(event Collision|EventActorBeginOverlap
  (params (OtherActor :type Actor%20Object%20Reference)))

(event EventTick
  (params (DeltaSeconds :type Float%20%28single-precision%29))
  (Variables|Default|GetHeldBuilding
    (:then
      (switch Utilities|FlowControl|Switch|SwitchonE_GameState (Variables|Default|GetCurrentGameState)
        (:NewEnumerator1
          (CallFunction|UpdateCursorBuildingPosition))))
    (:else)))

(fn ConstructionScript)

(fn GetGridStartLocation
  (return (- (Transformation|GetActorLocation) (Math|Vector|MakeVector (/ (* (Variables|Default|GetWidth) (Variables|Default|GetSellSize)) 2.0) (/ (* (Variables|Default|GetHeight) (Variables|Default|GetSellSize)) 2.0) 0.0))))

(fn WorldtoGrid
  (params (WorldPosition :type Vector))
  (bind _returnvalue (CallFunction|GetGridStartLocation))
  (bind _returnvalue_2 (- WorldPosition _returnvalue))
  (return (Utilities|Struct|MakeIntPoint (Math|Float|Floor (/ (.x _returnvalue_2) (Variables|Default|GetSellSize))) (Math|Float|Floor (/ (.y _returnvalue_2) (Variables|Default|GetSellSize))))))

(fn GridtoWorld
  (params (Grid :type Int%20Point%20Structure))
  (return (+ (CallFunction|GetGridStartLocation) (Math|Vector|MakeVector (+ (* (.x Grid) (Variables|Default|GetSellSize)) (/ (Variables|Default|GetSellSize) 2.0)) (+ (* (.y Grid) (Variables|Default|GetSellSize)) (/ (Variables|Default|GetSellSize) 2.0)) 0.0))))

(fn IsValidCoordinate
  (params (GridCoord :type Int%20Point%20Structure))
  (return (Math|Boolean|ANDBoolean (>= (.x GridCoord) 0) (>= (.y GridCoord) 0) (< (.x GridCoord) (Variables|Default|GetWidth)) (< (.y GridCoord) (Variables|Default|GetHeight)))))

(fn GetCellatGridCoordinate
  (params (GridCoord :type Int%20Point%20Structure))
  (bind (_x _y) (Utilities|Struct|BreakIntPoint GridCoord))
  (if (CallFunction|IsValidCoordinate GridCoord)
    (LocalVariables|SetIndex (+ _x (* _y (Variables|Default|GetWidth))))
    (if (and (>= (LocalVariables|GetIndex) 0) (<= (LocalVariables|GetIndex) (Utilities|Array|Length (Variables|Default|GetGridCell))))
      (return (Utilities|Array|Get(acopy) (Variables|Default|GetGridCell) (LocalVariables|GetIndex))))))

(fn GetCellatWorldPosition
  (params (WorldPosition :type Vector))
  (return (CallFunction|GetCellatGridCoordinate (CallFunction|WorldtoGrid WorldPosition))))

(fn InitalizeGrid
  (for _index (range 0 (- (Variables|Default|GetHeight) 1))
    (LocalVariables|SetY _index)
    (for _index_2 (range 0 (- (Variables|Default|GetWidth) 1))
      (LocalVariables|SetX _index_2)
      (bind _returnvalue (Game|SpawnActorfromClass "/Game/RaccoonСapitalists/Blueprints/BuildingSystem/BP_Cell.BP_Cell_C" (Math|Transform|MakeTransform (CallFunction|GridtoWorld (Utilities|Struct|MakeIntPoint (LocalVariables|GetX) (LocalVariables|GetY))) "0, 0, 0" "1.000000,1.000000,1.000000") "Undefined" "MultiplyWithRoot" 0 0))
      (Variables|/Game/RaccoonСapitalists/Blueprints/BuildingSystem/BP_Cell.BP_Cell_C|SetGridCoord _returnvalue (Utilities|Struct|MakeIntPoint (LocalVariables|GetX) (LocalVariables|GetY)))
      (Utilities|Array|Add (Variables|Default|GetGridCell) _returnvalue))))

(fn ClearHightlight
  (for _array_element (Variables|Default|GetPreviewslyHighlightCell)
    (Default|SetCellState _array_element "NewEnumerator0"))
  (Utilities|Array|Clear (Variables|Default|GetPreviewslyHighlightCell)))

(fn ValidateandHighlightPlacement
  (params (GridOrigin :type Int%20Point%20Structure) (FootPrint :type Array%20of%20Int%20Point%20Structures))
  (LocalVariables|SetOrigin GridOrigin)
  (LocalVariables|SetPrintFoot FootPrint)
  (switch Utilities|FlowControl|Switch|SwitchonE_GameState (Variables|Default|GetCurrentGameState)
    (:NewEnumerator1
      (CallFunction|ClearHightlight)
      (LocalVariables|SetCanPlace true)
      (for _array_element (LocalVariables|GetPrintFoot)
        (bind _output_get (LocalVariables|SetCoord (+ _array_element (LocalVariables|GetOrigin))))
        (if (not (CallFunction|IsValidCoordinate _output_get))
          (LocalVariables|SetCanPlace false)
          (else
            (Utilities|IsValid (CallFunction|GetCellatGridCoordinate (LocalVariables|GetCoord))
              (:Is%20Valid
                (Utilities|Array|Add (LocalVariables|GetCellToHighlight) (CallFunction|GetCellatGridCoordinate (LocalVariables|GetCoord)))
                (if (Variables|/Game/RaccoonСapitalists/Blueprints/BuildingSystem/BP_Cell.BP_Cell_C|GetisOccupided (CallFunction|GetCellatGridCoordinate (LocalVariables|GetCoord)))
                  (LocalVariables|SetCanPlace false)))))))
      (if (LocalVariables|GetCanPlace)
        (LocalVariables|SetHighlight "NewEnumerator1")
        (else
          (LocalVariables|SetHighlight "NewEnumerator2")))
      (for _array_element_2 (LocalVariables|GetCellToHighlight)
        (Default|SetCellState _array_element_2 (LocalVariables|GetHighlight))
        (Utilities|Array|Add (Variables|Default|GetPreviewslyHighlightCell) _array_element_2))
      (return (LocalVariables|GetCanPlace)))))

(fn CommitBuildingtoGrid
  (bind _heldbuilding (Variables|Default|GetHeldBuilding)
    (:then
      (LocalVariables|SetCurrentCell (CallFunction|GetCellatWorldPosition (Transformation|GetActorLocation _heldbuilding)))
      (for _array_element (Default|GetFootPrint (Variables|Default|GetHeldBuilding))
        (LocalVariables|SetCoord (+ _array_element (Variables|/Game/RaccoonСapitalists/Blueprints/BuildingSystem/BP_Cell.BP_Cell_C|GetGridCoord (LocalVariables|GetCurrentCell))))
        (if (CallFunction|IsValidCoordinate (+ _array_element (Variables|/Game/RaccoonСapitalists/Blueprints/BuildingSystem/BP_Cell.BP_Cell_C|GetGridCoord (LocalVariables|GetCurrentCell))))
          (Default|SetOccupided (CallFunction|GetCellatGridCoordinate (LocalVariables|GetCoord)) true)))
      (CallFunction|ClearHightlight)
      (Default|SetSolidBuildingMaterial (Variables|Default|GetHeldBuilding))
      (Default|ResourceGeneration (Variables|Default|GetHeldBuilding))
      (Variables|Default|SetCurrentGameState "NewEnumerator0"))
    (:else)))

(fn RotateHeldBuilding
  (bind _heldbuilding (Variables|Default|GetHeldBuilding))
  (bind _returnvalue (Transformation|GetActorRotation _heldbuilding))
  (bind _heldbuilding_2 (Variables|Default|GetHeldBuilding)
    (:then
      (Variables|/Game/RaccoonСapitalists/Blueprints/BuildingSystem/BP_Building.BP_Building_C|SetCurrentRotation _heldbuilding_2 (Math|Integer|%(Integer) (+ (Variables|/Game/RaccoonСapitalists/Blueprints/BuildingSystem/BP_Building.BP_Building_C|GetCurrentRotation _heldbuilding_2) 90) 360))
      (Transformation|SetActorRotation _heldbuilding (Math|Rotator|MakeRotator (.roll _returnvalue) (.pitch _returnvalue) (+ (.yaw _returnvalue) 9e+01)))
      (CallFunction|ValidateandHighlightPlacement (Variables|/Game/RaccoonСapitalists/Blueprints/BuildingSystem/BP_Cell.BP_Cell_C|GetGridCoord (CallFunction|GetCellatWorldPosition (Transformation|GetActorLocation (Variables|Default|GetHeldBuilding)))) (Default|GetFootPrint (Variables|Default|GetHeldBuilding))))
    (:else)))

(fn CanCelCurrentAction
  (switch Utilities|FlowControl|Switch|SwitchonE_GameState (Variables|Default|GetCurrentGameState)
    (:NewEnumerator1
      (bind _heldbuilding (Variables|Default|GetHeldBuilding)
        (:then
          (Actor|DestroyActor _heldbuilding)
          (Variables|Default|SetHeldBuilding 0)
          (CallFunction|ClearHightlight))
        (:else)))
    (:NewEnumerator2
      (bind _selectbuilding (Variables|Default|GetSelectBuilding)
        (:then
          (Default|SetSelected _selectbuilding false)
          (Variables|Default|SetSelectBuilding 0))
        (:else))))
  (Variables|Default|SetCurrentGameState "NewEnumerator0"))

(fn SelectBuildingonGrid
  (params (TargetBuilding :type BP%20Building%20Object%20Reference))
  (Utilities|IsValid TargetBuilding
    (:Is%20Valid
      (CallFunction|CanCelCurrentAction)
      (bind _output_get (Variables|Default|SetSelectBuilding TargetBuilding))
      (Default|SetSelected _output_get true)
      (Variables|Default|SetCurrentGameState "NewEnumerator2"))))

(fn DeselectBuilding
  (bind _selectbuilding (Variables|Default|GetSelectBuilding)
    (:then
      (Default|SetSelected _selectbuilding false)
      (Variables|Default|SetSelectBuilding 0)
      (Variables|Default|SetCurrentGameState "NewEnumerator0"))
    (:else)))

(fn DeleteSelectBuilding
  (bind _selectbuilding (Variables|Default|GetSelectBuilding)
    (:then
      (LocalVariables|SetCell (CallFunction|GetCellatWorldPosition (Transformation|GetActorLocation _selectbuilding)))
      (for _array_element (Default|GetFootPrint (Variables|Default|GetSelectBuilding))
        (Default|SetOccupided (CallFunction|GetCellatGridCoordinate (+ _array_element (Variables|/Game/RaccoonСapitalists/Blueprints/BuildingSystem/BP_Cell.BP_Cell_C|GetGridCoord (LocalVariables|GetCell)))) false))
      (Actor|DestroyActor (Variables|Default|GetSelectBuilding))
      (Variables|Default|SetSelectBuilding 0)
      (Variables|Default|SetCurrentGameState "NewEnumerator0"))
    (:else)))

(fn UpdateCursorBuildingPosition
  (bind _returnvalue (Game|GetPlayerController 0))
  (bind _returnvalue_2 (Game|GetPlayerController 0))
  (bind (_locationx _locationy) (Game|Player|GetMousePosition _returnvalue))
  (bind (_worldposition _worlddirection) (Class|GameplayStatics|DeprojectScreentoWorld _returnvalue_2 (Math|Vector2D|MakeVector2D _locationx _locationy)))
  (Variables|Default|GetHeldBuilding
    (:then
      (switch Utilities|FlowControl|Switch|SwitchonE_GameState (Variables|Default|GetCurrentGameState)
        (:NewEnumerator1
          (bind _outhit (Collision|LineTraceByChannel _worldposition (+ _worldposition (* _worlddirection 5e+04)) "TraceTypeQuery1" false 0 "None"))
          (Utilities|IsValid (CallFunction|GetCellatWorldPosition (.location _outhit))
            (:Is%20Valid
              (bind _output_get (LocalVariables|SetHitCell (CallFunction|GetCellatWorldPosition (.location _outhit))))
              (Transformation|SetActorLocation (Variables|Default|GetHeldBuilding) (CallFunction|GridtoWorld (Variables|/Game/RaccoonСapitalists/Blueprints/BuildingSystem/BP_Cell.BP_Cell_C|GetGridCoord _output_get)) false false)
              (CallFunction|ValidateandHighlightPlacement (Variables|/Game/RaccoonСapitalists/Blueprints/BuildingSystem/BP_Cell.BP_Cell_C|GetGridCoord (LocalVariables|GetHitCell)) (Default|GetFootPrint (Variables|Default|GetHeldBuilding))))))))
    (:else)))

(fn SpawnandAttachBuilding
  (params (class :type BP%20Building%20Class%20Reference) (BuildingType :type E_BuildingType%20Enum :default "NewEnumerator0"))
  (LocalVariables|SetType BuildingType)
  (CallFunction|CanCelCurrentAction)
  (bind _returnvalue (Game|SpawnActorfromClass class (Math|Transform|MakeTransform "0, 0, 0" "0, 0, 0" "1.000000,1.000000,1.000000") "Undefined" "MultiplyWithRoot" 0 0))
  (bind _output_get (Variables|Default|SetHeldBuilding _returnvalue))
  (Variables|/Game/RaccoonСapitalists/Blueprints/BuildingSystem/BP_Building.BP_Building_C|SetBuildingType _output_get (LocalVariables|GetType))
  (Variables|/Game/RaccoonСapitalists/Blueprints/BuildingSystem/BP_Building.BP_Building_C|SetCurrentRotation _output_get 0)
  (Variables|Default|SetCurrentGameState "NewEnumerator1")
  (CallFunction|UpdateCursorBuildingPosition))

(fn HandleLeftClick
  (bind _returnvalue (Game|GetPlayerController 0))
  (bind _returnvalue_2 (Game|GetPlayerController 0))
  (bind (_locationx _locationy) (Game|Player|GetMousePosition _returnvalue))
  (bind (_worldposition _worlddirection) (Class|GameplayStatics|DeprojectScreentoWorld _returnvalue_2 (Math|Vector2D|MakeVector2D _locationx _locationy)))
  (switch Utilities|FlowControl|Switch|SwitchonE_GameState (Variables|Default|GetCurrentGameState)
    (:NewEnumerator0
      (bind _outhit (Collision|LineTraceByChannel _worldposition (+ _worldposition (* _worlddirection 5e+04)) "TraceTypeQuery1" false 0 "None"))
      (bind _asbp_building (Utilities|Casting|CastToBP_Building (.hitactor _outhit)))
      (CallFunction|SelectBuildingonGrid _asbp_building))
    (:NewEnumerator1
      (bind _heldbuilding (Variables|Default|GetHeldBuilding)
        (:then
          (Utilities|IsValid (CallFunction|GetCellatWorldPosition (Transformation|GetActorLocation _heldbuilding))
            (:Is%20Valid
              (bind _canplace1 (CallFunction|ValidateandHighlightPlacement (Variables|/Game/RaccoonСapitalists/Blueprints/BuildingSystem/BP_Cell.BP_Cell_C|GetGridCoord (CallFunction|GetCellatWorldPosition (Transformation|GetActorLocation _heldbuilding))) (Default|GetFootPrint (Variables|Default|GetHeldBuilding))))
              (if _canplace1
                (CallFunction|CommitBuildingtoGrid)))))
        (:else)))
    (:NewEnumerator2
      (CallFunction|CanCelCurrentAction))))

(fn HandleRightClick
  (CallFunction|CanCelCurrentAction))

(fn HandleRotateKey
  (switch Utilities|FlowControl|Switch|SwitchonE_GameState (Variables|Default|GetCurrentGameState)
    (:NewEnumerator1
      (CallFunction|RotateHeldBuilding))))

(fn HandleDelete
  (switch Utilities|FlowControl|Switch|SwitchonE_GameState (Variables|Default|GetCurrentGameState)
    (:NewEnumerator2
      (CallFunction|DeleteSelectBuilding))))